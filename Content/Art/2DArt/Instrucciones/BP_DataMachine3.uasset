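; Instruction-art actor with a plane whose "notas" material fades in and out according to a travel value (Recorrido).
; The construction script creates a dynamic material instance for the plane and sets its starting OpacityLevel.
; IncreaseOpacity maps Recorrido through Min, Peak and Min2, ramping opacity up to full at Peak, back down toward Min2, and zeroing it outside that range.
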(event Custom|IncreaseOpacity
  (params (recorrido :type Float%20%28double-precision%29))
  (if (and (< recorrido (Variables|Default|Getpeak)) (>= recorrido (Variables|Default|Getmin)))
    (Rendering|Material|SetScalarParameterValue (Variables|Default|GetNotasMat) "OpacityLevel" (Math|Float|MapRangeClamped recorrido (Variables|Default|Getmin) (Variables|Default|Getpeak) 0.0 1.0) :!class /Script/Engine.MaterialInstanceDynamic)
    (elif (and (< recorrido (Variables|Default|Getmin2)) (>= recorrido (Variables|Default|Getpeak)))
      (Rendering|Material|SetScalarParameterValue (Variables|Default|GetNotasMat) "OpacityLevel" (Math|Float|MapRangeClamped recorrido (Variables|Default|Getpeak) (Variables|Default|Getmin2) 1.0 0.0) :!class /Script/Engine.MaterialInstanceDynamic)
      (else
        (Rendering|Material|SetScalarParameterValue (Variables|Default|GetNotasMat) "OpacityLevel" 0.0 :!class /Script/Engine.MaterialInstanceDynamic)))))

(event EventBeginPlay)

(event Collision|EventActorBeginOverlap
  (params (OtherActor :type Actor%20Object%20Reference)))

(event EventTick
  (params (DeltaSeconds :type Float%20%28single-precision%29)))

(fn ConstructionScript
  (bind _returnvalue (Rendering|Material|CreateDynamicMaterialInstance (Rendering|Material|GetMaterial (Variables|Default|GetPlane) 0) "None" "None" :!class /Script/Engine.KismetMaterialLibrary))
  (bind _output_get (Variables|Default|SetNotasMat _returnvalue))
  (Rendering|Material|SetMaterial (Variables|Default|GetPlane) 0 _output_get)
  (Rendering|Material|SetScalarParameterValue (Variables|Default|GetNotasMat) "OpacityLevel" (Variables|Default|Getopacity) :!class /Script/Engine.MaterialInstanceDynamic))